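; BP_SmallSphere is a short-lived moving sphere actor that tumbles as it travels, then shrinks or scales away and destroys itself.
; On BeginPlay it picks a random roll-free rotation rate and starts a lifetime timer.
; Each Tick offsets it along its forward vector and rotates it, so the spin continually bends its path.
; When the timer fires, the WinkOut timeline drives the mesh's uniform scale, destroying the actor when finished.
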(event Custom|WinkOut
  (bind _scale (Timeline|WinkOutTimeline Play)
    (:Update
      (CallFunction|ScaleSphere _scale))
    (:Finished
      (Actor|DestroyActor))))

(event EventBeginPlay
  (CallFunction|InitializeDeltaRotation)
  (Utilities|Time|SetTimerbyEvent (delegate Custom|WinkOut) (Variables|Default|GetLifetime)))

(event EventTick
  (params (DeltaSeconds :type Float%20%28single-precision%29))
  (CallFunction|UpdateLocation DeltaSeconds)
  (CallFunction|UpdateRotation))

(fn ConstructionScript)

(fn InitializeDeltaRotation
  (Variables|SphereMovement|SetRotationSpeed (* (Math|Random|RandomRotator false) (Variables|SphereMovement|GetRotationScaleFactor))))

(fn UpdateLocation
  (params (DeltaTime :type Float%20%28double-precision%29))
  (Transformation|AddActorWorldOffset (* (* DeltaTime (Variables|SphereMovement|GetSpeed)) (Transformation|GetActorForwardVector))))

(fn UpdateRotation
  (Class|Actor|AddActorWorldRotation (* (Variables|SphereMovement|GetRotationSpeed) (Utilities|Time|GetWorldDeltaSeconds))))

(fn ScaleSphere
  (params (Scale :type Float%20%28single-precision%29))
  (Transformation|SetWorldScale3D (Variables|Default|GetSphereMesh) (Math|Vector|MakeVector Scale Scale Scale)))